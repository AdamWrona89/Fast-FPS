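; Enemy spawner actor that periodically populates the level with BP_BaseEnemy instances.
; On BeginPlay it starts a looping timer that calls SpawnEnemy every few seconds.
; Each tick checks the CurrentEnemies count on GS_FastFps and, while under a fixed cap, spawns an enemy at a random navigable point around the world origin.
; The navmesh used for that query comes from the game state's RecastNavmesh reference.
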(event Custom|SpawnEnemy
  (bind _asgs_fast_fps (Utilities|Casting|CastToGS_FastFps (Game|GetGameState)))
  (if (< (Utilities|Array|Length (Variables|/Game/GameMode/GS_FastFps.GS_FastFps_C|GetCurrentEnemies _asgs_fast_fps)) 10)
    (bind _asgs_fast_fps_2 (Utilities|Casting|CastToGS_FastFps (Game|GetGameState)))
    (Game|SpawnActorfromClass "/Game/Enemy/BP_BaseEnemy.BP_BaseEnemy_C" (Math|Transform|MakeTransform (.RandomLocation (Class|NavigationSystemV1|GetRandomPointinNavigableRadius (Math|Vector|MakeVector 0.0 0.0 0.0) 2.5e+03 (Variables|/Game/GameMode/GS_FastFps.GS_FastFps_C|GetRecastNavmesh _asgs_fast_fps_2) 0)) "0, 0, 0" "1,1,1") "Undefined" 0 0)))

(event EventBeginPlay
  (Utilities|Time|SetTimerbyFunctionName 0 "SpawnEnemy" 5.0 true))

(fn ConstructionScript)